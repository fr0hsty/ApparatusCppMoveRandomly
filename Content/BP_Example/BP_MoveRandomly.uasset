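; Example Blueprint that demonstrates ECS-style subjects, traits and mechanics by moving subjects between random points on a flat plane.
; BeginPlay spawns the subjects with random position and destination traits.
; Each Tick, one mechanic moves subjects toward their destinations and tags arrivals with a finished-movement trait.
; A separate mechanic gives tagged subjects new destinations and removes the tag, keeping responsibilities split, while two more draw debug points for positions and destinations.
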(event `self.ReceiveBeginPlay`
  (bind _returnvalue (* (* (`KismetMathLibrary.RandomUnitVector`) (`self.RandomSpawnWidth`)) (1.0 1.0 0.0)))
  (for _ (range (+ (`self.NumSubjects`) 1))
    (bind _outsubjecthandle (`ApparatusFunctionLibrary.SpawnMachineSubject` 0)) ; Create a new subject
    (`|ExecutionSequence`
      (:`then_0`
        (`|SetSubjectTrait` _outsubjecthandle "/Game/BP_Example/Traits/FBPDestination.FBPDestination" (make `/Game/BP_Example/Traits/FBPDestination` _returnvalue)) ; Gvie it a destination
      )
      (:`then_1`
        (`|SetSubjectTrait` _outsubjecthandle "/Game/BP_Example/Traits/FBPSubjectPosition.FBPSubjectPosition" (make `/Game/BP_Example/Traits/FBPSubjectPosition` _returnvalue)) ; Give it a position
      ))))

(event `self.ReceiveTick`
  (params (DeltaSeconds :type "Float (single-precision)"))
  (`|ExecutionSequence`
    (:`then_0`
      (bind (_subject _subjective _trait_0 _trait_1) (`|Mechanic` "/Game/BP_Example/Traits/FBPSubjectPosition.FBPSubjectPosition" "/Game/BP_Example/Traits/FBPDestination.FBPDestination")
        (:`Operate`
          (bind _value (break `/Game/BP_Example/Traits/FBPDestination` _trait_1))
          (bind _value_2 (break `/Game/BP_Example/Traits/FBPSubjectPosition` _trait_0))
          (if (>= (`KismetMathLibrary.Vector_Distance` _value _value_2) (`self.MinDistanceToDestination`))
            (`|SetSubjectTrait` _subject "/Game/BP_Example/Traits/FBPSubjectPosition.FBPSubjectPosition" (make `/Game/BP_Example/Traits/FBPSubjectPosition` (+ (* (* (`KismetMathLibrary.Normal` (- _value _value_2)) (`GameplayStatics.GetWorldDeltaSeconds`)) (`self.SubjectMovespeed`)) _value_2))) ; Update the subjects position trait
            (else
              ;[1 1 1] Flag this subject as someone who has finished movement for a seperate mechanic to handle.
              ;
              ; NOTE - You don't have to do this, you could just handle getting a new random destination right here and setting it ... BUT that would mean that this mechanic is responsible for several things (moving AND finding a new location when finished moving).
              ;
              ; It might be appropriate for you to structure your mechanics so that they take care of small and specific pieces of logic, which you can then slowly begin to structure all of your game logic arround.
              ;
              ; I personally would NOT do this in the event that a mechanic must iterate over many many subjects multiple times, this could be slow when dealing with several hundred thousand subjects. But for when subjects "finish" moving? There won't be many in the game world at any one time.
              (`|SetSubjectTrait` _subject "/Game/BP_Example/Traits/FBPFinishedMovement.FBPFinishedMovement" (make `/Game/BP_Example/Traits/FBPFinishedMovement` false)) ; Flag this subject as someone who has finished movement for other mechanics to handle
            )))))
    (:`then_1`
      (bind _subject_2 (`|Mechanic` "/Game/BP_Example/Traits/FBPFinishedMovement.FBPFinishedMovement") ; Find destinations for all subjects waiting for them
        (:`Operate`
          (`|SetSubjectTrait` _subject_2 "/Game/BP_Example/Traits/FBPDestination.FBPDestination" (make `/Game/BP_Example/Traits/FBPDestination` (* (* (`KismetMathLibrary.RandomUnitVector`) (1.0 1.0 0.0)) (`self.RandomSpawnWidth`))))
          (`ApparatusFunctionLibrary.RemoveSubjectTrait` _subject_2 "/Game/BP_Example/Traits/FBPFinishedMovement.FBPFinishedMovement"))))
    (:`then_2`
      (bind (_subject_3 _subjective_2 _trait_0_2) (`|Mechanic` "/Game/BP_Example/Traits/FBPSubjectPosition.FBPSubjectPosition")
        (:`Operate`
          (`KismetSystemLibrary.DrawDebugPoint` (`.Value_2_46D0B3754FCB6F913AD782B2A376446F` (break `/Game/BP_Example/Traits/FBPSubjectPosition` _trait_0_2)) 20.0 (struct :`G` 1.0 :`A` 1.0)))))
    (:`then_3`
      (bind (_subject_4 _subjective_3 _trait_0_3) (`|Mechanic` "/Game/BP_Example/Traits/FBPDestination.FBPDestination")
        (:`Operate`
          (`KismetSystemLibrary.DrawDebugPoint` (`.Value_2_46D0B3754FCB6F913AD782B2A376446F` (break `/Game/BP_Example/Traits/FBPDestination` _trait_0_3)) 20.0 (struct :`R` 1.0 :`A` 1.0)))))))

(fn `UserConstructionScript`)